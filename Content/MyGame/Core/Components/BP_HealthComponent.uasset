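; Health component that tracks a character's HP, resets it each round and records who dealt damage.
; The server fills HP at BeginPlay, and damage subtracts from it, clamping at zero and calling Dead, whose body is empty here.
; CurrentHP uses a RepNotify to update the owning player's HUD health bar and rounded-up text, which also refresh on possession.
; The character death call sits in disconnected nodes and never runs.
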(event `Possesed`
  (bind _currenthp (`self.CurrentHP`))
  (bind _mainhudref (`/Game/MyGame/Core/Gameplay/Gameplay_PC.MainHudRef` (`/Game/MyGame/Characters/MainCharacter.PlayerControllerRef` (`self.CharacterRef`))))
  ;[1 1 1] Possesed
  (`/Engine/EditorBlueprintResources/StandardMacros.IsValid` _mainhudref
    (:`Is Valid`
      (`ProgressBar.SetPercent` (`/Game/MyGame/UI/Gameplay/Widget_MainHud.ProgressBar_Health` _mainhudref) (`KismetMathLibrary.NormalizeToRange` _currenthp 0.0 (`self.MaxHP`)))
      (`TextBlock.SetText` (`/Game/MyGame/UI/Gameplay/Widget_MainHud.Text_Health` _mainhudref) (`KismetTextLibrary.Conv_Int64ToText` (`KismetMathLibrary.FCeil64` _currenthp))))))

(event `self.ReceiveBeginPlay`
  ;[1 1 1] Begin Play
  (`parent.ReceiveBeginPlay`)
  (if (`KismetSystemLibrary.IsServer`)
    (`self.SetMaxHp`)))

(event `GetDamage`
  (params (Damage :type "Float (double-precision)") (Causer :type "Actor Object Reference"))
  ;[1 1 1] Get Damage
  (`KismetArrayLibrary.Array_AddUnique` (`self.DamageCausers`) Causer)
  (set `self.LastDamageCauser` Causer)
  (bind _output_get (set `self.CurrentHP` (- (`self.CurrentHP`) Damage)))
  (if (<= _output_get 0.0)
    (set `self.CurrentHP` 0.0)
    (`self.Dead`)))

(event `SetMaxHP`
  ;[1 1 1] Max HP
  (set `self.CurrentHP` (`self.MaxHP`)))

(event `Dead`)

(event `NewRound`
  ;[1 1 1] New Round
  (`self.SetMaxHP`)
  (`KismetArrayLibrary.Array_Clear` (`self.DamageCausers`))
  (set `self.LastDamageCauser` null))

(fn `OnRep_CurrentHP`
  (bind _currenthp (`self.CurrentHP`))
  (bind _playercontrollerref (`/Game/MyGame/Characters/MainCharacter.PlayerControllerRef` (`self.CharacterRef`)))
  (bind _mainhudref (`/Game/MyGame/Core/Gameplay/Gameplay_PC.MainHudRef` _playercontrollerref))
  (`/Engine/EditorBlueprintResources/StandardMacros.IsValid` _playercontrollerref
    (:`Is Valid`
      (`/Engine/EditorBlueprintResources/StandardMacros.IsValid` _mainhudref
        (:`Is Valid`
          (`ProgressBar.SetPercent` (`/Game/MyGame/UI/Gameplay/Widget_MainHud.ProgressBar_Health` _mainhudref) (`KismetMathLibrary.NormalizeToRange` _currenthp 0.0 (`self.MaxHP`)))
          (`TextBlock.SetText` (`/Game/MyGame/UI/Gameplay/Widget_MainHud.Text_Health` _mainhudref) (`KismetTextLibrary.Conv_Int64ToText` (`KismetMathLibrary.FCeil64` _currenthp))))))))