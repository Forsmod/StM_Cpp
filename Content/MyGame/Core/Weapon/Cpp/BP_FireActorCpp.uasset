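; BP_FireActorCpp is a weapon-related fire actor Blueprint that cleans itself up when the level is cleared.
; On BeginPlay, the authority binds its Destroy event to the Gameplay_GM_Cpp game mode's clear-level event.
; Destroy removes the actor only if its current player is invalid or dead, so weapons of living players survive the clear.
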(event `self.ReceiveBeginPlay`
  (`parent.ReceiveBeginPlay`)
  (`/Engine/EditorBlueprintResources/ActorMacros.Switch Has Authority`
    (:`Authority`
      (bind _asgameplay_gm_cpp (cast `/Game/MyGame/Core/CPP/Gameplay_GM_Cpp` (`GameplayStatics.GetGameMode`)))
      (add `/Game/MyGame/Core/CPP/Gameplay_GM_Cpp.ClearLevel` _asgameplay_gm_cpp (delegate `Destroy`)))))

(event `Destroy`
  (bind _currentplayer (`self.CurrentPlayer`))
  (`/Engine/EditorBlueprintResources/StandardMacros.IsValid` _currentplayer
    (:`Is Valid`
      (if (`GameplayCharacterCpp.bIsDead` _currentplayer)
        (`self.K2_DestroyActor` :!label _label)))
    (:`Is Not Valid`
      (goto _label))))

(fn `UserConstructionScript`)