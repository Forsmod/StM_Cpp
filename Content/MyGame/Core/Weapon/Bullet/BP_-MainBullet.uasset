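; BP_-MainBullet is a weapon projectile that damages actors and leaves bullet holes on surfaces.
; Box overlaps ignore the owner and actors of the instigator's class; otherwise they apply damage on the server only, spawn a half-scale blood effect and destroy the bullet.
; Box hits spawn a BP_Bullet_Hole at the impact point, oriented to the surface normal, then destroy the bullet.
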(event `self.Box.OnComponentBeginOverlap`
  (params (OverlappedComponent :type "PrimitiveComponent Object Reference") (OtherActor :type "Actor Object Reference") (OtherComp :type "PrimitiveComponent Object Reference") (OtherBodyIndex :type Integer) (bFromSweep :type Boolean) (SweepResult :type "HitResult Structure (by ref)"))
  (bind _returnvalue (`self.GetInstigator`))
  (set `self.SweepPoint` SweepResult_Location)
  (bind _output_get (set `self.Other Actor` OtherActor))
  (if (== (`GameplayStatics.GetObjectClass` _output_get) (`GameplayStatics.GetObjectClass` (`self.GetInstigator`)))
    _
    (elif (not (== (`self.Other Actor`) (`self.GetOwner`)))
      (if (`KismetSystemLibrary.IsServer`)
        (`GameplayStatics.ApplyDamage` (`self.Other Actor`) (`self.Damage`) (`Pawn.GetController` _returnvalue) _returnvalue))
      (`GameplayStatics.SpawnEmitterAtLocation` "/Game/MyGame/FX/P_Blood.P_Blood" (`self.SweepPoint`) (struct) (0.5 0.5 0.5))
      (`self.K2_DestroyActor`))))

(event `self.Box.OnComponentHit`
  (params (HitComponent :type "PrimitiveComponent Object Reference") (OtherActor :type "Actor Object Reference") (OtherComp :type "PrimitiveComponent Object Reference") (NormalImpulse :type "Vector Structure") (Hit :type "HitResult Structure (by ref)"))
  (`|SpawnActorFromClass` "/Game/MyGame/Core/Weapon/Bullet/BP_Bullet_Hole.BP_Bullet_Hole_C" (`KismetMathLibrary.MakeTransform` Hit_ImpactPoint (`KismetMathLibrary.Conv_VectorToRotator` Hit_ImpactNormal)) "Undefined" "OverrideRootScale" null null)
  (`self.K2_DestroyActor`))

(fn `UserConstructionScript`)