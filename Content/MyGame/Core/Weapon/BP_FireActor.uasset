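; Firearm weapon actor that handles looped or single-shot firing, ammo and timed reloading for the current player.
; A gated loop macro paces shots by fire rate and feeds a reload macro that spends ammo or auto-reloads when empty.
; Each shot traces from the player's camera to aim the muzzle at the crosshair target, then multicasts the AK47 bullet spawn, muzzle effect and sound, and shakes the camera.
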(event `self.ReceiveBeginPlay`
  (`parent.ReceiveBeginPlay`)
  (set `self.AttackSpeed` (/ 1.0 (`KismetMathLibrary.Conv_IntToDouble` (`self.AttackSpeed/Sec`)))))

(event `self.StartFire`
  (bind _followcamera (`/Game/MyGame/Characters/MainCharacter.FollowCamera` (`self.CurrentPlayer`)))
  (bind _followcamera_2 (`/Game/MyGame/Characters/MainCharacter.FollowCamera` (`self.CurrentPlayer`)))
  (bind _returnvalue (`SceneComponent.K2_GetComponentLocation` _followcamera_2))
  (`self.M_LoopFire` :!label _label
    (:`Fire`
      (`/Engine/EditorBlueprintResources/StandardMacros.IsValid` (`self.CurrentPlayer`)
        (:`Is Valid`
          (`self.M_Reload` :!label _label_2
            (:`Out`
              (`self.UpdateWidget` (`self.WeaponStats`))
              (bind (_outhit _returnvalue_2) (`KismetSystemLibrary.CapsuleTraceSingle` _returnvalue (+ _returnvalue (* (`SceneComponent.GetForwardVector` _followcamera_2) 10000)) 0.0 0.0 "TraceTypeQuery1" false (`|MakeArray` (`self.CurrentPlayer`) :!type "Actor Object Reference")))
              (if _returnvalue_2
                (bind _outtransform (`self.BulletTransform` (`.ImpactPoint` (`GameplayStatics.BreakHitResult` _outhit))))
                (set `self.TansformBullet` _outtransform)
                (else
                  (bind _outtransform_2 (`self.BulletTransform` (+ (`SceneComponent.K2_GetComponentLocation` _followcamera) (* (`SceneComponent.GetForwardVector` _followcamera) 10000))))
                  (set `self.TansformBullet` _outtransform_2)))
              (`self.SpawnBullet_Multicast` (`self.TansformBullet`))
              (`/Game/MyGame/Characters/MainCharacter.ShakeCamera` (`self.CurrentPlayer`)))))
        (:`Is Not Valid`
          (goto _label :!via `EndFire`))))))

(event `SpawnBullet_Multicast`
  (params (SpawnTransform :type "Transform Structure"))
  (bind _returnvalue (`|SpawnActorFromClass` "/Game/MyGame/Core/Weapon/Bullet/BP_AK47Bullet.BP_AK47Bullet_C" SpawnTransform "Undefined" "OverrideRootScale" self (`self.CurrentPlayer`)))
  (set `/Game/MyGame/Core/Weapon/Bullet/BP_-MainBullet.Damage` (`self.Damage`) _returnvalue)
  (`GameplayStatics.SpawnEmitterAttached` "/Game/MyGame/FX/P_Explosion.P_Explosion" (`self.BulletStart`) "None" (0.0 0.0 0.0) (struct) (0.2 0.2 0.2))
  (`GameplayStatics.SpawnSoundAtLocation` "/Game/MyGame/Audio/Shoots_Cue.Shoots_Cue" (.location SpawnTransform) (struct) 1.0 1.0 0.0 null null))

(event `self.EndFire`
  (goto _label :!via `EndFire`))

(event `Reload`
  (bind (_weaponstats_currentammo _weaponstats_maxammoinclip) (break `/Game/MyGame/Core/Weapon/ST_WeaponInfo` (`self.WeaponStats`)))
  ;[1 1 1] Reload
  (if (!= _weaponstats_currentammo _weaponstats_maxammoinclip)
    (goto _label_2 :!via `Reload`)))

(fn `BulletTransform`
  (params (Target :type "Vector Structure (by ref)"))
  (returns (OutTransform :type "Transform Structure"))
  (bind _returnvalue (`SceneComponent.K2_GetComponentLocation` (`self.BulletStart`)))
  (return (`KismetMathLibrary.MakeTransform` _returnvalue (`KismetMathLibrary.FindLookAtRotation` _returnvalue Target))))

(fn `UserConstructionScript`
  (`parent.UserConstructionScript`))