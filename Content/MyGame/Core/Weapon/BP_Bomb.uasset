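; Bomb weapon for a team round mode: Ch_RedTeam characters pick it up and plant it, Ch_BlueTeam characters defuse it.
; Planting and defusing are interruptible timers that lock movement and fire, with a DoOnce admitting one defuser.
; Planting spawns an armed copy, removes the held weapon and flags Gameplay_GM.
; Detonation applies distance-scaled damage to actors overlapping its box; either detonation or defusal ends the round.
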(event `self.Capsule.OnComponentBeginOverlap`
  (params (OverlappedComponent :type "PrimitiveComponent Object Reference") (OtherActor :type "Actor Object Reference") (OtherComp :type "PrimitiveComponent Object Reference") (OtherBodyIndex :type Integer) (bFromSweep :type Boolean) (SweepResult :type "HitResult Structure (by ref)"))
  (`/Engine/EditorBlueprintResources/ActorMacros.Switch Has Authority`
    (:`Authority`
      (bind _asmain_character (cast `/Game/MyGame/Characters/MainCharacter` OtherActor))
      (if (== (`GameplayStatics.GetObjectClass` _asmain_character) "/Game/MyGame/Characters/Ch_RedTeam.Ch_RedTeam_C")
        (bind _bp_weaponcomponent (`/Game/MyGame/Characters/MainCharacter.BP_WeaponComponent` _asmain_character))
        (if (not (`/Game/MyGame/Core/Components/BP_WeaponComponent.SlotValid?` _bp_weaponcomponent (`self.WeaponType`)))
          (`/Game/MyGame/Core/Components/BP_WeaponComponent.AddWeaponServer` _bp_weaponcomponent self))))))

(event `self.EndFire`
  ;[1 1 1] Stop Planting
  (`KismetSystemLibrary.K2_ClearAndInvalidateTimerHandle` (`self.SetTimer`))
  (`self.SetCharacterMovementAndFire` (`self.CurrentPlayer`) true
    (:`Out`
      (`self.PrintOwningClient` "Stop Planting Bomb"))))

(event `self.StartFire`
  ;[1 1 1] Planting
  (if (`/Game/MyGame/Characters/MainCharacter.IsOnThePlant?` (`self.CurrentPlayer`))
    (`self.SetCharacterMovementAndFire` (`self.CurrentPlayer`)
      (:`Out`
        (bind _returnvalue (`KismetSystemLibrary.K2_SetTimerDelegate` (delegate `SetTimerE`) (`self.TimeToPlant`)))
        (set `self.SetTimer` _returnvalue)
        (`self.PrintOwningClient` "Start Planting Bomb")))))

(event `SetTimerE`
  (bind _bp_weaponcomponent (`/Game/MyGame/Characters/MainCharacter.BP_WeaponComponent` (`self.CurrentPlayer`)))
  ;[1 1 1] Plant
  (if (`/Game/MyGame/Characters/MainCharacter.IsOnThePlant?` (`self.CurrentPlayer`))
    (`self.SetCharacterMovementAndFire` (`self.CurrentPlayer`) true
      (:`Out`
        (bind _returnvalue (`|SpawnActorFromClass` (`GameplayStatics.GetObjectClass` self) (`KismetMathLibrary.MakeTransform` (`self.K2_GetActorLocation` (`self.CurrentPlayer`)) (struct :`Roll` 90.0)) "AdjustIfPossibleButAlwaysSpawn" "OverrideRootScale" null null))
        (`PrimitiveComponent.SetCollisionResponseToChannel` (`/Game/MyGame/Core/Weapon/BP_WeaponActor.Capsule` _returnvalue) "ECC_Pawn" "ECR_Ignore")
        (`self.SetBomb` _returnvalue)
        (`/Game/MyGame/Core/Components/BP_WeaponComponent.RemoveWeaponServer` _bp_weaponcomponent (`GameplayStatics.GetObjectClass` self))
        (`/Game/MyGame/Core/Components/BP_WeaponComponent.SelectValidWeaponServer` _bp_weaponcomponent)
        (`self.K2_DestroyActor`)))))

(event `SetBomb`
  (bind _returnvalue (`KismetSystemLibrary.K2_SetTimerDelegate` (delegate `Boom`) (`self.TimeToExplosion`)))
  (set `self.BombTimer` _returnvalue)
  (`self.PrintMulticast` "Bomb Has Been Planted")
  (bind _asgameplay_gm (cast `/Game/MyGame/Core/Gameplay/Gameplay_GM` (`GameplayStatics.GetGameMode`)))
  (set `/Game/MyGame/Core/Gameplay/Gameplay_GM.BombIsPlanted?` true _asgameplay_gm))

(event `Boom`
  (bind _box (`self.Box`))
  ;[1 1 1] Boom
  (`/Game/MyGame/Core/Gameplay/Gameplay_GM.RoundEnd` (cast `/Game/MyGame/Core/Gameplay/Gameplay_GM` (`GameplayStatics.GetGameMode`) :!pure true) true)
  (`self.SpawnEmmiter`)
  (`PrimitiveComponent.SetCollisionEnabled` _box "QueryOnly")
  (for _array_element (`PrimitiveComponent.GetOverlappingActors` _box null)
    (`GameplayStatics.ApplyDamage` _array_element (`KismetMathLibrary.MapRangeClamped` (`self.GetDistanceTo` _array_element) 1000.0 2500.0 200.0)))
  (`KismetSystemLibrary.Delay` 0.2)
  (`self.K2_DestroyActor`))

(event `SpawnEmmiter`
  ;[1 1 1] Boom
  (`GameplayStatics.SpawnEmitterAtLocation` "/Game/MyGame/FX/P_Explosion.P_Explosion" (`self.K2_GetActorLocation`) (struct) (20.0 20.0 20.0)))

(event `BreakDefusingServer`
  (params (Character :type "/Game/MyGame/Characters/MainCharacter Object Reference"))
  (if (== Character (`self.DefuserRef`))
    (`/Game/MyGame/Characters/MainCharacter.PrintOwningClient` (`self.DefuserRef`) "Stop Defusing Bomb")
    (`KismetSystemLibrary.K2_ClearAndInvalidateTimerHandle` (`self.BombDefusingTimer`))
    (`self.SetCharacterMovementAndFire` (`self.DefuserRef`) true
      (:`Out`
        (set `self.DefuserRef` null)
        (goto _label :!via `Reset`)))))

(event `StartDefusingBombServer`
  (params (Character :type "/Game/MyGame/Characters/MainCharacter Object Reference"))
  (if (== (`GameplayStatics.GetObjectClass` Character) "/Game/MyGame/Characters/Ch_BlueTeam.Ch_BlueTeam_C")
    (`/Engine/EditorBlueprintResources/StandardMacros.DoOnce` false :!label _label
      (:`Completed`
        (set `self.DefuserRef` Character)
        (bind _returnvalue (`KismetSystemLibrary.K2_SetTimerDelegate` (delegate `BombDefusedServer`) (`self.TimeToDefuse`)))
        (set `self.BombDefusingTimer` _returnvalue)
        (`/Game/MyGame/Characters/MainCharacter.PrintOwningClient` (`self.DefuserRef`) "Start Defusing Bomb")
        (`self.SetCharacterMovementAndFire` (`self.DefuserRef`))))))

(event `BombDefusedServer`
  ;[1 1 1] Defuse
  (`KismetSystemLibrary.K2_ClearAndInvalidateTimerHandle` (`self.BombTimer`))
  (`PrimitiveComponent.SetCollisionResponseToChannel` (`self.Capsule`) "ECC_Visibility" "ECR_Ignore")
  (`self.PrintMulticast` "Bomb has been defused")
  (`/Game/MyGame/Core/Gameplay/Gameplay_GM.RoundEnd` (cast `/Game/MyGame/Core/Gameplay/Gameplay_GM` (`GameplayStatics.GetGameMode`) :!pure true) false)
  (`self.SetCharacterMovementAndFire` (`self.DefuserRef`) true))

(fn `UserConstructionScript`)