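; Throwable grenade weapon that explodes on a three-second fuse, dealing radial damage with falloff.
; StartFire hands off to the player's weapon component; Throw launches the physics capsule along the owner's camera direction, inheriting the owner's velocity.
; After the fuse, authority applies damage, calls the explosion effect event, then destroys the actor.
; Authority also feeds capsule location and velocity into SynchronizeMoveGrenade every tick to keep the physics motion in sync.
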(event `self.StartFire`
  (`/Game/MyGame/Core/Components/BP_WeaponComponent.ThrowGrenade` (`/Game/MyGame/Characters/MainCharacter.BP_WeaponComponent` (`self.CurrentPlayer`))))

(event `Throw`
  (bind _returnvalue (`self.GetOwner`))
  (bind _returnvalue_2 (`SceneComponent.K2_GetComponentLocation` (`self.Capsule`)))
  (`PrimitiveComponent.SetCollisionEnabled` (`self.Capsule`) "PhysicsOnly")
  (`PrimitiveComponent.SetPhysicsLinearVelocity` (`self.Capsule`) (+ (* (`SceneComponent.GetForwardVector` (`/Game/MyGame/Characters/MainCharacter.FollowCamera` (cast `/Game/MyGame/Characters/MainCharacter` (`self.GetOwner`) :!pure true))) 1500) (`self.GetVelocity` (`self.GetOwner`))) false "None")
  (`KismetSystemLibrary.Delay` 3.0)
  (`/Engine/EditorBlueprintResources/ActorMacros.Switch Has Authority`
    (:`Authority`
      (`GameplayStatics.ApplyRadialDamageWithFalloff` :`BaseDamage` 50.0 :`Origin` _returnvalue_2 :`DamageInnerRadius` 200.0 :`DamageOuterRadius` 1000.0 :`DamageFalloff` 2.0 :`DamageCauser` _returnvalue :`InstigatedByController` (`self.GetInstigatorController` _returnvalue) :`DamagePreventionChannel` "ECC_Pawn")
      (`self.SpawnExplosion` _returnvalue_2)
      (`KismetSystemLibrary.Delay` 0.2)
      (`self.K2_DestroyActor`))))

(event `SpawnExplosion`
  (params (Location :type "Vector Structure"))
  (`GameplayStatics.SpawnEmitterAtLocation` "/Game/MyGame/FX/P_Explosion.P_Explosion" Location (struct) (5.0 5.0 5.0)))

(event `self.ReceiveTick`
  (params (DeltaSeconds :type "Float (single-precision)"))
  (bind _capsule (`self.Capsule`))
  ;[1 1 1] SynchronizeMove
  (`/Engine/EditorBlueprintResources/ActorMacros.Switch Has Authority`
    (:`Authority`
      (bind _returnvalue (`PrimitiveComponent.GetPhysicsLinearVelocity` _capsule "None"))
      (`self.SynchronizeMoveGrenade` (`SceneComponent.K2_GetComponentLocation` _capsule) _returnvalue))))

(event `SynchronizeMoveGrenade`
  (params (Location :type "Vector Structure") (Velocity :type "Vector Structure"))
  (bind _capsule (`self.Capsule`))
  ;[1 1 1] SynchronizeMove
  (`SceneComponent.K2_SetWorldLocation` _capsule Location false false)
  (`PrimitiveComponent.SetPhysicsLinearVelocity` _capsule Velocity false "None"))

(fn `UserConstructionScript`
  (`parent.UserConstructionScript`))