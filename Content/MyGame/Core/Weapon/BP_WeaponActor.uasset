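; Base weapon actor that characters pick up by overlap and that can be dropped, with empty StartFire and EndFire events.
; The authority adds it to the character's weapon component when that slot check fails, and registers Destroy with the game mode's level clear.
; Destroy refills the clip and HUD for living owners, otherwise removes the actor.
; Once dropped, a looping timer synchronizes capsule transform and velocity until it rests, then disables physics.
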(event `PrintMulticast`
  (params (InString :type String))
  ;[1 1 1] Print
  (`KismetSystemLibrary.PrintString` InString true true (struct :`R` 1.0 :`A` 1.0) 5.0))

(event `PrintOwningClient`
  (params (InString :type String))
  ;[1 1 1] Print
  (`KismetSystemLibrary.PrintString` InString true true (struct :`R` 1.0 :`A` 1.0) 5.0))

(event `self.ReceiveBeginPlay`
  (`/Engine/EditorBlueprintResources/ActorMacros.Switch Has Authority`
    (:`Authority`
      (bind _asgameplay_gm (cast `/Game/MyGame/Core/Gameplay/Gameplay_GM` (`GameplayStatics.GetGameMode`)))
      (add `/Game/MyGame/Core/Gameplay/Gameplay_GM.ClearLevel` _asgameplay_gm (delegate `Destroy`)))))

(event `Destroy`
  (bind _currentplayer (`self.CurrentPlayer`))
  (bind _weaponstats (`self.WeaponStats`))
  (`/Engine/EditorBlueprintResources/StandardMacros.IsValid` _currentplayer
    (:`Is Valid`
      (if (`/Game/MyGame/Characters/MainCharacter.IsDead?` _currentplayer)
        (`self.K2_DestroyActor` :!label _label)
        (else
          (bind _structout (setmembers `/Game/MyGame/Core/Weapon/ST_WeaponInfo` :`StructRef` _weaponstats :`CurrentAmmo` (`.MaxAmmoInClip_11_A958D95D40DFA7E25E799F8643F1800E` (break `/Game/MyGame/Core/Weapon/ST_WeaponInfo` _weaponstats))))
          (`self.UpdateWidget` _structout))))
    (:`Is Not Valid`
      (goto _label))))

(event `UpdateWidget`
  (params (WeaponInfo :type "/Game/MyGame/Core/Weapon/ST_WeaponInfo Structure"))
  (bind _currentplayer (`self.CurrentPlayer`))
  ;[1 1 1] Update Wiget Ammo
  (`/Engine/EditorBlueprintResources/StandardMacros.IsValid` _currentplayer
    (:`Is Valid`
      (bind _asgameplay_pc (cast `/Game/MyGame/Core/Gameplay/Gameplay_PC` (`Pawn.GetController` _currentplayer)))
      (`/Game/MyGame/UI/Gameplay/Widget_MainHud.UpdateWidgetAmmo` (`/Game/MyGame/Core/Gameplay/Gameplay_PC.MainHudRef` _asgameplay_pc) WeaponInfo (`self.Name`)))))

(event `self.Capsule.OnComponentBeginOverlap`
  (params (OverlappedComponent :type "PrimitiveComponent Object Reference") (OtherActor :type "Actor Object Reference") (OtherComp :type "PrimitiveComponent Object Reference") (OtherBodyIndex :type Integer) (bFromSweep :type Boolean) (SweepResult :type "HitResult Structure (by ref)"))
  (`/Engine/EditorBlueprintResources/ActorMacros.Switch Has Authority`
    (:`Authority`
      (bind _asmain_character (cast `/Game/MyGame/Characters/MainCharacter` OtherActor))
      (bind _bp_weaponcomponent (`/Game/MyGame/Characters/MainCharacter.BP_WeaponComponent` _asmain_character))
      (if (not (`/Game/MyGame/Core/Components/BP_WeaponComponent.SlotValid?` _bp_weaponcomponent (`self.WeaponType`)))
        (`/Game/MyGame/Core/Components/BP_WeaponComponent.AddWeaponServer` _bp_weaponcomponent self)))))

(event `StartFire`)

(event `EndFire`)

(event `Droped`
  (bind _returnvalue (`KismetSystemLibrary.K2_SetTimerDelegate` (delegate `PhysicsTick`) 0.1 true))
  (set `self.TimerPhysics` _returnvalue))

(event `PhysicsTick`
  (bind _capsule (`self.Capsule`))
  (bind _returnvalue (`SceneComponent.K2_GetComponentLocation` _capsule))
  (bind _returnvalue_2 (`PrimitiveComponent.GetPhysicsLinearVelocity` _capsule "None"))
  (`self.SynchronizeMove` (`SceneComponent.K2_GetComponentToWorld` _capsule) _returnvalue_2)
  (if (== _returnvalue (`self.OldPosition`) :`ErrorTolerance` 0.1)
    (`KismetSystemLibrary.K2_ClearAndInvalidateTimerHandle` (`self.TimerPhysics`))
    (`self.DisableSynchronizeMove`)
    (else
      (set `self.OldPosition` _returnvalue))))

(event `SynchronizeMove`
  (params (Transform :type "Transform Structure") (Velocity :type "Vector Structure"))
  (`SceneComponent.K2_SetWorldTransform` (`self.Capsule`) Transform false false)
  (`PrimitiveComponent.SetPhysicsLinearVelocity` (`self.Capsule`) Velocity false "None"))

(event `DisableSynchronizeMove`
  (`PrimitiveComponent.SetSimulatePhysics` (`self.Capsule`) false))

(fn `UserConstructionScript`)