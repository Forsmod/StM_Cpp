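; Weapon spawner that places an evenly spaced row of weapon actors along its forward axis.
; The construction script sizes the spawn area and previews the row with instanced meshes, which are destroyed at BeginPlay.
; On the server, a self-retriggering DoN loop spawns and records up to MaxWeapon weapons.
; RespawnAll, registered with Gameplay_GM for level clearing, empties the array without destroying actors and reruns the loop.
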(event `self.ReceiveBeginPlay`
  (`ActorComponent.K2_DestroyComponent` (`self.HierarchicalInstancedStaticMesh`))
  (`/Engine/EditorBlueprintResources/ActorMacros.Switch Has Authority`
    (:`Authority`
      (bind _asgameplay_gm (cast `/Game/MyGame/Core/Gameplay/Gameplay_GM` (`GameplayStatics.GetGameMode`)))
      (add `/Game/MyGame/Core/Gameplay/Gameplay_GM.ClearLevel` _asgameplay_gm (delegate `RespawnAll`))
      (bind _counter (`/Engine/EditorBlueprintResources/StandardMacros.Do N` (`self.MaxWeapon`) :!label _label)
        (:`Exit`
          (`self.Respawn` _counter)
          (goto _label))))))

(event `RespawnAll`
  (`KismetArrayLibrary.Array_Clear` (`self.WeaponArray`))
  (`|ExecutionSequence`
    (:`then_0`
      (goto _label :!via `Reset`))
    (:`then_1`
      (goto _label))))

(fn `Respawn`
  (params (Count :type Integer))
  (bind _defaultsceneroot (`self.DefaultSceneRoot`))
  (bind (_returnvalue_roll _returnvalue_pitch _returnvalue_yaw) (`KismetMathLibrary.BreakRotator` (`SceneComponent.K2_GetComponentRotation` _defaultsceneroot)))
  (bind _returnvalue (`|SpawnActorFromClass` (`self.Weapon`) (`KismetMathLibrary.MakeTransform` (+ (* (`SceneComponent.GetForwardVector` _defaultsceneroot) (* (- Count 1) (`self.Distance`))) (`SceneComponent.K2_GetComponentLocation` _defaultsceneroot)) (`KismetMathLibrary.MakeRotator` _returnvalue_roll _returnvalue_pitch (- _returnvalue_yaw 180.0))) "AdjustIfPossibleButDontSpawnIfColliding" "OverrideRootScale" self null))
  (`KismetArrayLibrary.Array_Add` (`self.WeaponArray`) _returnvalue))

(fn `UserConstructionScript`
  (bind _returnvalue (`KismetMathLibrary.Conv_IntToDouble` (* (- (`self.MaxWeapon`) 1) (/ (`self.Distance`) 2))))
  (`BoxComponent.SetBoxExtent` (`self.SpawnArea`) (`KismetMathLibrary.MakeVector` _returnvalue 50.0 50.0) false)
  (`SceneComponent.K2_SetRelativeLocation` (`self.SpawnArea`) (`KismetMathLibrary.MakeVector` _returnvalue) false false)
  (for _index (range 1 (+ (`self.MaxWeapon`) 1))
    (`InstancedStaticMeshComponent.AddInstance` (`self.HierarchicalInstancedStaticMesh`) (`KismetMathLibrary.MakeTransform` (* (1.0 0.0 0.0) (* (- _index 1) (`self.Distance`))) (struct :`Pitch` 90.0 :`Yaw` 90.0) (2.0 2.0 2.0)))))